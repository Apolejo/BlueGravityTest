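; Main skateboarding player character Blueprint, handling the push-off animation and jump/score UI feedback.
; StartSpeeding plays the speeding-start montage once until ResetSpeeding, holding StartMovement false until a montage notify begins.
; On BeginPlay it caches the WBP_ChargeJump from its UICharge widget component, which charge events use to update the progress bar.
; Score events update that widget's text and spawn a BP_Widget_Score actor just above the hit location.
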(event `self.ReceiveBeginPlay`
  (`self.CastToChargeJump`))

(event `self.StartSpeeding`
  ;[1 1 1] AnimationMontageStartMovement
  (`/Engine/EditorBlueprintResources/StandardMacros.DoOnce` false :!label _label
    (:`Completed`
      (set `self.StartMovement` false)
      (`|PlayMontage` (`self.Mesh`) "/Game/Content_Skateboard/Assets/Animations/Player/AM_Skateboard_Speeding_Start.AM_Skateboard_Speeding_Start"
        (:`OnNotifyBegin`
          (set `self.StartMovement` true))))))

(event `self.ResetSpeeding`
  ;[1 1 1] AnimationMontageStartMovement
  (goto _label :!via `Reset`))

(event `self.BPEvent_OnSpawnScore`
  (params (HitLocation :type "Vector Structure") (ScoreTotal :type Integer))
  ;[1 1 1] JumpedOverObstacle
  (`/Game/Content_Skateboard/UserInterface/WBP_ChargeJump.UpdateText` (`self.Ref_ChargeJump`) (`KismetTextLibrary.Conv_IntToText` ScoreTotal))
  (`|SpawnActorFromClass` "/Game/Content_Skateboard/Blueprints/UserInterface/BP_Widget_Score.BP_Widget_Score_C" (`KismetMathLibrary.MakeTransform` (+ HitLocation (0.0 0.0 50.0))) "Undefined" "MultiplyWithRoot" null null))

(event `self.BPEvent_OnChargeJump`
  (params (Charge :type "Float (single-precision)"))
  ;[1 1 1] JumpCharge
  (`/Game/Content_Skateboard/UserInterface/WBP_ChargeJump.SetProgressBar` (`self.Ref_ChargeJump`) Charge))

(fn `CastToChargeJump`
  (bind _aswbp_charge_jump (cast `/Game/Content_Skateboard/UserInterface/WBP_ChargeJump` (`WidgetComponent.GetWidget` (`self.UI_Charge`))))
  (set `self.Ref_ChargeJump` _aswbp_charge_jump))

(fn `UserConstructionScript`)